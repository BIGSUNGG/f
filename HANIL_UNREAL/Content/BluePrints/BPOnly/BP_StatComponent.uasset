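; BP_StatComponent is a stat component that holds an owner's Level, Attack, Hp and MaxHp.
; On BeginPlay it sets level 1, pulling that level's stats from BP_MyGameInstance and filling Hp to max.
; Damage routes through SetHp, which clamps Hp between zero and MaxHp and notifies subscribers of the new ratio through the HpChanged delegate.
; Helper functions expose the Hp ratio, current and max Hp, and death state.
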(event `self.ReceiveBeginPlay`
  (`self.SetLevel` 1))

(fn `Damaged`
  (params (amount :type Integer))
  ;[1 1 1] Attack 받았을 때
  (`self.SetHp` (- (`self.Hp`) amount)))

(fn `GetCurHp`
  (returns (CurHp :type "Float (double-precision)"))
  (return (`KismetMathLibrary.Conv_IntToDouble` (`self.Hp`))))

(fn `GetHpRatio`
  (returns (HpRatio :type "Float (double-precision)"))
  ;[1 1 1] Hp Ratio 구하기
  (return (/ (`KismetMathLibrary.Conv_IntToDouble` (`self.Hp`)) (`KismetMathLibrary.Conv_IntToDouble` (`self.MaxHp`)))))

(fn `GetMaxHp`
  (returns (MaxHp :type "Float (double-precision)"))
  (return (`KismetMathLibrary.Conv_IntToDouble` (`self.MaxHp`))))

(fn `IsDead`
  (returns (IsDead :type Boolean))
  (if (<= (`self.Hp`) 0)
    (return true)
    (else
      (return false))))

(fn `SetHp`
  (params (ChangedHp :type Integer))
  ;[1 1 1] SetHp...(설정하려는 Hp가 0보다 작거나, MaxHp보다 클 때 맞춰주기 위한 예외처리), 체력이 바뀌었을 때 구독자들에게 알려주기(Delegate)
  (bind _output_get (set `self.Hp` ChangedHp))
  (if (< _output_get 0)
    (set `self.Hp` 0))
  (if (> (`self.Hp`) (`self.MaxHp`))
    (set `self.Hp` (`self.MaxHp`)))
  (bind _hpratio (`self.GetHpRatio`))
  (`self.HpChanged` _hpratio))

(fn `SetLevel`
  (params (level :type Integer))
  ;[1 1 1] Level를 입력해서 Stat정보 받아오기
  (bind _asbp_my_game_instance (cast `/Game/BluePrints/BPOnly/BP_MyGameInstance` (`GameplayStatics.GetGameInstance`)))
  (bind _newparam (`/Game/BluePrints/BPOnly/BP_MyGameInstance.GetStatDataByLevel` _asbp_my_game_instance level))
  (bind (_level _attack _maxhp) (break `/Game/BluePrints/BPOnly/MyCharacterData` _newparam))
  (set `self.Level` _level)
  (set `self.Attack` _attack)
  (set `self.MaxHp` _maxhp)
  (`self.SetHp` _maxhp))